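; Fan actor Blueprint that spins the lower part of a fan on demand.
; Start Fan Rotation targets a Rotating Movement component at FanLowerPart, applies the RotationRate variable and activates it.
; End Fan Rotation stops the movement immediately and deactivates the component.
; The construction script is empty, and nothing in the graphs shown calls either function.
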(fn `End Fan Rotation`
  (bind _rotatingmovement (`self.RotatingMovement`))
  (`MovementComponent.StopMovementImmediately` _rotatingmovement)
  (`ActorComponent.Deactivate` _rotatingmovement))

(fn `Start Fan Rotation`
  (`MovementComponent.SetUpdatedComponent` (`self.RotatingMovement`) (`self.Fan_LowerPart`))
  (set `RotatingMovementComponent.RotationRate` (`self.Rotation Rate`) (`self.RotatingMovement`))
  (`ActorComponent.Activate` (`self.RotatingMovement`) false))

(fn `UserConstructionScript`)