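; BP_Clock shows one digit of the current time on a plane, as seconds, minutes, 12-hour or 24-hour hours.
; The construction script creates a dynamic material instance from Clock_MI.
; Each Tick reads the unit chosen by NumberType and uses string operations to extract the ones or tens place chosen by Digit.
; That digit indexes SegTexture to set the material's Display texture.
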(event `self.ReceiveTick`
  (params (DeltaSeconds :type "Float (single-precision)"))
  (bind (_returnvalue_year _returnvalue_month _returnvalue_day _returnvalue_hour _returnvalue_minute _returnvalue_second) (`KismetMathLibrary.BreakDateTime` (`KismetMathLibrary.Now`)))
  (bind _returnvalue (`KismetMathLibrary.Now`))
  (bind _returnvalue_2 (`KismetStringLibrary.Conv_IntToString` (`self.Time`)))
  (bind _returnvalue_3 (`KismetStringLibrary.GetCharacterArrayFromString` _returnvalue_2))
  (switch `/Game/Blueprints/Clock/DigitSelection` (`self.NumberType`)
    (:`NewEnumerator0`
      (set `self.Time` _returnvalue_second))
    (:`NewEnumerator1`
      (set `self.Time` _returnvalue_minute))
    (:`NewEnumerator2`
      (set `self.Time` (`KismetMathLibrary.GetHour12` _returnvalue)))
    (:`NewEnumerator3`
      (set `self.Time` (`KismetMathLibrary.GetHour` _returnvalue))))
  (switch `int` (`self.Digit`)
    (:`0`
      (`MaterialInstanceDynamic.SetTextureParameterValue` (`self.SegMaterial`) "Display" (`|GetArrayItem` (`self.SegTexture`) (`KismetMathLibrary.FTrunc` (`KismetStringLibrary.Conv_StringToDouble` (`|GetArrayItem` _returnvalue_3 (`KismetArrayLibrary.Array_LastIndex` _returnvalue_3)))))))
    (:`1`
      (`MaterialInstanceDynamic.SetTextureParameterValue` (`self.SegMaterial`) "Display" (`|GetArrayItem` (`self.SegTexture`) (`KismetMathLibrary.FTrunc` (`KismetStringLibrary.Conv_StringToDouble` (`KismetStringLibrary.LeftChop` _returnvalue_2 1))))))))

(fn `UserConstructionScript`
  (bind _returnvalue (`PrimitiveComponent.CreateDynamicMaterialInstance` (`self.Plane`) 0 "/Game/Blueprints/Clock/Material/Clock_MI.Clock_MI" "None"))
  (set `self.SegMaterial` _returnvalue))