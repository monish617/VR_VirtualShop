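; FanSwitchBoard_BP is a switch board that lets the player turn a linked TargetFan on and off.
; FanStatusInfo writes a click or touch prompt to the given HUD, and FanInteraction flips FanStatus and starts or ends the fan's rotation.
; FanStatus names the next action rather than the current state, so ON means the next interaction starts the fan.
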(event `/Game/Interaction/Interactables.Fan Status Info`
  (params (HUD :type "/Game/Blueprints/HUD/WB/Interactive_Dot/Interactive_Status_info Object Reference"))
  (switch `/Game/Interaction/FanState` (`self.FanStatus`)
    (:`NewEnumerator0`
      (`/Game/Blueprints/HUD/WB/Interactive_Dot/Interactive_Status_info.Set  info` HUD "Click / Touch  To Turn ON Fan"))
    (:`NewEnumerator1`
      (`/Game/Blueprints/HUD/WB/Interactive_Dot/Interactive_Status_info.Set  info` HUD "Click / Touch  To Turn OFF Fan"))))

(event `/Game/Interaction/Interactables.Fan Interaction`
  (bind _target_fan (`self.Target_Fan`))
  (switch `/Game/Interaction/FanState` (`self.FanStatus`)
    (:`NewEnumerator0`
      (set `self.FanStatus` "NewEnumerator1")
      (`/Game/Blueprints/Fan_BP.Start Fan Rotation` _target_fan))
    (:`NewEnumerator1`
      (set `self.FanStatus` "NewEnumerator0")
      (`/Game/Blueprints/Fan_BP.End Fan Rotation` _target_fan))))

(fn `UserConstructionScript`)