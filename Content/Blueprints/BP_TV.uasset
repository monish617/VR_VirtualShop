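; BP_TV is an interactable television that starts and stops a video and shows a matching click/touch prompt on the HUD.
; TvInteraction flips TVState, either opening the virtual shop media source on the PlayMedia player or closing it.
; ShowTvInfo reads the same state to set the HUD text.
; The state naming is inverted: On means the TV is ready to switch on, so interacting then opens the media and sets Off.
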(event `/Game/Interaction/Interactables.TvInteraction`
  (bind _playmedia (`self.PlayMedia`))
  ;[0.5016 1 0.4099] Tv Interaction
  (switch `/Game/Interaction/TvState` (`self.TVState`)
    (:`NewEnumerator0`
      (set `self.TVState` "NewEnumerator1")
      (`MediaPlayer.OpenSource` _playmedia "/Game/Movies/virtual_shop_renderd0001-1407.virtual_shop_renderd0001-1407"))
    (:`NewEnumerator1`
      (set `self.TVState` "NewEnumerator0")
      (`MediaPlayer.Close` _playmedia))))

(event `/Game/Interaction/Interactables.Show Tv Info`
  (params (Hud :type "/Game/Blueprints/HUD/WB/Interactive_Dot/Interactive_Status_info Object Reference"))
  ;[0.5016 1 0.4099] Tv Status
  (switch `/Game/Interaction/TvState` (`self.TVState`)
    (:`NewEnumerator0`
      (`/Game/Blueprints/HUD/WB/Interactive_Dot/Interactive_Status_info.Set  info` Hud "Click / Touch  to On the Tv"))
    (:`NewEnumerator1`
      (`/Game/Blueprints/HUD/WB/Interactive_Dot/Interactive_Status_info.Set  info` Hud "Click / Touch To Off The Tv"))))

(fn `UserConstructionScript`)