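; Inspectable product actor that the player clicks or taps to examine up close along with its brand, size, price and material.
; A do-once click handler moves input from the character to the actor, attaches it to the camera manager, slides it into view and shows a Display_Details widget.
; Mouse axes rotate the root during inspection.
; IA_Cancel detaches it, restores character input, removes the widget and returns it to its saved transform.
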(event `self.ReceiveBeginPlay`
  (set `self.As BP My Player Controller` (cast `/Game/Blueprints/BP_MyPlayerController` (`GameplayStatics.GetPlayerController` 0) :!pure true)))

(event `self.ReceiveActorOnClicked`
  (params (ButtonPressed :type "Key Structure"))
  (bind _returnvalue (`GameplayStatics.GetPlayerController` 0))
  (bind _defaultsceneroot (`self.DefaultSceneRoot`))
  (`self.DisableInput` (`GameplayStatics.GetPlayerCharacter` 0) _returnvalue :!label _label)
  (`self.EnableInput` _returnvalue)
  (`/Engine/EditorBlueprintResources/StandardMacros.DoOnce` false :!label _label_2
    (:`Completed`
      (set `self.Original Transform` (`self.GetTransform`))
      (set `self.actor clicked` true)
      (set `self.Inspecting?` true)
      (`self.K2_AttachToComponent` self (`PlayerCameraManager.TransformComponent` (`GameplayStatics.GetPlayerCameraManager` 0)) "None" "KeepWorld" "KeepWorld" "KeepWorld" true)
      (`KismetSystemLibrary.MoveComponentTo` _defaultsceneroot (50.0 28.0 -6.0) (`SceneComponent.RelativeRotation` _defaultsceneroot) false false 0.3)
      (`self.EnableInput` (`GameplayStatics.GetPlayerController` 0))
      (`self.ToggleDisplayDetails` true))))

(event `self.ReceiveActorOnInputTouchBegin`
  (params (FingerIndex :type "ETouchIndex Enum" :default "Touch1"))
  (goto _label))

(event `self.StaticMesh.OnClicked`
  (params (TouchedComponent :type "PrimitiveComponent Object Reference") (ButtonPressed :type "Key Structure"))
  (goto _label))

(event `EnhancedInput|/Game/ThirdPerson/Input/Actions/IA_Cancel`
  (params (ActionValue :type Boolean) (ElapsedSeconds :type "Float (double-precision)") (TriggeredSeconds :type "Float (double-precision)") (InputAction :type "InputAction Object Reference" :default "/Game/ThirdPerson/Input/Actions/IA_Cancel.IA_Cancel"))
  (bind _returnvalue (`GameplayStatics.GetPlayerController` 0))
  (:`Started`
    (if (`self.actor clicked`)
      (`self.DisableInput` _returnvalue)
      (`self.EnableInput` (`GameplayStatics.GetPlayerCharacter` 0) _returnvalue)
      (set `self.Inspecting?` false)
      (`self.K2_DetachFromActor` self "KeepWorld" "KeepWorld" "KeepWorld")
      (`self.ToggleDisplayDetails` false)
      (`KismetSystemLibrary.MoveComponentTo` (`self.DefaultSceneRoot`) (.location (`self.Original Transform`)) (.rotation (`self.Original Transform`)))
      (goto _label_2 :!via `Reset`))))

(event `InputAxis|Turn Right / Left Mouse`
  (params (AxisValue :type "Float (single-precision)"))
  (`SceneComponent.K2_AddLocalRotation` (`self.DefaultSceneRoot`) (`KismetMathLibrary.MakeRotator` 0.0 0.0 AxisValue) false false))

(event `InputAxis|Look Up / Down Mouse`
  (params (AxisValue :type "Float (single-precision)"))
  (`SceneComponent.K2_AddLocalRotation` (`self.DefaultSceneRoot`) (`KismetMathLibrary.MakeRotator` AxisValue) false false))

(fn `ToggleDisplayDetails`
  (params (`Enable/Disable` :type Boolean))
  (bind _displaydetails (`self.Displaydetails`))
  (if `Enable/Disable`
    (`/Engine/EditorBlueprintResources/StandardMacros.IsValid` (`self.Displaydetails`)
      (:`Is Valid`
        _)
      (:`Is Not Valid`
        _))
    (bind _returnvalue (`|CreateWidget` "/Game/Blueprints/Inspection/Display_Details.Display_Details_C" (`GameplayStatics.GetPlayerController` 0)))
    (bind _output_get (set `self.Displaydetails` _returnvalue))
    (`/Game/Blueprints/Inspection/Display_Details.Initialize_Details` _output_get (`self.Brand Name`) (`self.Size`) (`self.Price`) (`self.Material`))
    (`UserWidget.AddToViewport` _output_get 0)
    (else
      (`/Engine/EditorBlueprintResources/StandardMacros.IsValid` _displaydetails
        (:`Is Valid`
          (`Widget.RemoveFromParent` _displaydetails))))))

(fn `UserConstructionScript`)