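; BP_MainDoor is an interactive door that swings open and shut and supplies a HUD prompt for the available action.
; DoorInteraction flips DoorStatus and plays or reverses a Timeline that lerps the static mesh's yaw between 0 and -90 degrees.
; DoorStatus names the next action rather than the current state, and ShowDoorInfo uses it to pick the prompt.
; TvInteraction is an empty stub.
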(event `/Game/Interaction/Interactables.DoorInteraction`
  ;[0.5016 1 0.4099] Door Interaction
  (switch `/Game/Interaction/DoorState` (`self.Door Status`)
    (:`NewEnumerator0`
      (set `self.Door Status` "NewEnumerator1")
      (bind (_direction _alpha) (`Timeline|Timeline` :!label _label)
        (:`Update`
          (`SceneComponent.K2_SetRelativeRotation` (`self.StaticMesh`) (`KismetMathLibrary.MakeRotator` 0.0 0.0 (`KismetMathLibrary.Lerp` 0.0 -90.0 _alpha)) false false))))
    (:`NewEnumerator1`
      (set `self.Door Status` "NewEnumerator0")
      (goto _label :!via `Reverse`))))

(event `/Game/Interaction/Interactables.Show Door Info`
  (params (HUD :type "/Game/Blueprints/HUD/WB/Interactive_Dot/Interactive_Status_info Object Reference"))
  ;[0.5016 1 0.4099] Show Door Status
  (switch `/Game/Interaction/DoorState` (`self.Door Status`)
    (:`NewEnumerator0`
      (`/Game/Blueprints/HUD/WB/Interactive_Dot/Interactive_Status_info.Set  info` HUD "Click / Touch  To Open The Door"))
    (:`NewEnumerator1`
      (`/Game/Blueprints/HUD/WB/Interactive_Dot/Interactive_Status_info.Set  info` HUD "Click / Touch  close the Door"))))

(event `/Game/Interaction/Interactables.TvInteraction`)

(fn `UserConstructionScript`)